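; Game mode for a Mars marine wave shooter that spawns escalating waves of aliens.
; Each wave multiplies and rounds the difficulty into a spawn count, then a looping timer spawns BP_Alien at random TargetPoints until that count is used up.
; Reported alien deaths shrink the tracked Aliens list; once none remain alive or pending, the next wave starts after a short delay.
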(event Custom|SpawnWave
  (CallFunction|SpawnAlien))

(event Custom|EndWave
  (Utilities|FlowControl|Delay 2.0)
  (CallFunction|StartNewWave))

(event EventBeginPlay
  (Utilities|FlowControl|Delay 2.0)
  (CallFunction|StartNewWave))

(fn ConstructionScript)

(fn StartNewWave
  (Math|Integer|IncrementInt (Variables|Default|GetCurrentWave)
    (:%20%20
      (CallFunction|IncreseWaveDifficulty)
      (Utilities|Time|SetTimerbyFunctionName 0 "SpawnWave" (Variables|Default|GetSpawn%20Frequency) true))))

(fn SpawnAlien
  (bind _spawnpoint (CallFunction|GetRandomSpawnPoint))
  (Utilities|IsValid _spawnpoint
    (:Is%20Valid
      (bind _returnvalue (Game|SpawnActorfromClass "/Game/Blueprints/AI/BP_Alien.BP_Alien_C" (Transformation|GetActorTransform _spawnpoint) "Undefined" 0 0))
      (Utilities|IsValid _returnvalue
        (:Is%20Valid
          (Utilities|Array|Add (Variables|Default|GetAliens) _returnvalue)
          (bind _result (Math|Integer|DecrementInt (Variables|Default|GetAliensSpawnRemaining))
            (:%20%20
              (if (== _result 0)
                (Utilities|Time|ClearTimerbyFunctionName 0 "SpawnWave")))))))))

(fn GetRandomSpawnPoint
  (bind _outactors (Actor|GetAllActorsOfClass "/Script/Engine.TargetPoint"))
  (return (Utilities|Array|Get(acopy) _outactors (Math|Random|RandomIntegerinRange 0 (Utilities|Array|LastIndex _outactors)))))

(fn RegisterAlienDeath
  (params (DeadAlien :type BP%20Alien%20Object%20Reference%20%28by%20ref%29))
  (Utilities|Array|RemoveItem (Variables|Default|GetAliens) DeadAlien)
  (if (CallFunction|IsWaveComplete)
    (CallFunction|EndWave)))

(fn IsWaveComplete
  (return (and (== (Utilities|Array|Length (Variables|Default|GetAliens)) 0) (== (Variables|Default|GetAliensSpawnRemaining) 0))))

(fn IncreseWaveDifficulty
  (bind _output_get (Variables|Default|SetWaveDifficulty (Math|Float|Round (* (Variables|Default|GetWaveDifficulty) (Variables|Default|GetDifficultyMultiplier)))))
  (Variables|Default|SetAliensSpawnRemaining _output_get))