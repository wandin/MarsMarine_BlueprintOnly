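; Player-controlled Marine for a twin-stick shooter, with world-axis movement, automatic rifle fire, health and a kill counter, shown with a W_PlayerHud widget.
; Each tick it smoothly turns control rotation toward mouse velocity or thumbstick direction beyond a dead zone, switching by last key pressed.
; Firing runs muzzle effects, looping sound and a repeating timer line trace that applies damage.
; Damage reduces health; zero sets Dead, blocking input and stopping fire.
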(event EventBeginPlay
  ;[1 0.9475 0.2806] Create Widget HUD
  (bind _returnvalue (UserInterface|CreateWidget "/Game/UI/W_PlayerHud.W_PlayerHud_C" 0 self))
  (UserInterface|Viewport|AddtoViewport _returnvalue 0))

(event Game|Damage|EventAnyDamage
  (params (Damage :type Float%20%28single-precision%29) (DamageType :type Damage%20Type%20Object%20Reference) (InstigatedBy :type Controller%20Object%20Reference) (DamageCauser :type Actor%20Object%20Reference))
  ;[1 0.07005 0.1398] Health Deduction when hit by the Alien
  (if (CallFunction|IsPlayerAlive)
    (bind _health (CallFunction|DecreaseHealth Damage))
    (if (== _health 0.0)
      (Variables|PlayerProperties|SetDead true)
      (CallFunction|StopFiringWeapon))))

(event EventTick
  (params (DeltaSeconds :type Float%20%28single-precision%29))
  ;[0.4001 1 0.288] Update Aim
  (CallFunction|UpdatePlayerAim))

(event Input|ActionEvents|InputActionFireWeapon
  (params (Key :type Key%20Structure :default "None"))
  ;[1 0.6016 0.5718] Fire weapon
  (:Pressed
    (CallFunction|StartFiringWeapon))
  (:Released
    (CallFunction|StopFiringWeapon)))

(event Input|AxisEvents|InputAxisMoveForward
  (params (AxisValue :type Float%20%28single-precision%29))
  ;[1 0.4225 0.912] Movement
  (if (CallFunction|IsPlayerAlive)
    (Pawn|Input|AddMovementInput "1.000000,0.000000, 0" AxisValue true)))

(event Input|AxisEvents|InputAxisMoveRight
  (params (AxisValue :type Float%20%28single-precision%29))
  ;[1 0.4225 0.912] Movement
  (if (CallFunction|IsPlayerAlive)
    (Pawn|Input|AddMovementInput "0,1.000000,0.000000" AxisValue true)))

(event Input|KeyboardEvents|AnyKey
  (params (Key :type Key%20Structure :default "None"))
  ;[0.4876 0.7731 1] Set GamePad or Mouse Control
  (:Pressed
    (Variables|Default|SetGamePadActive (Class|KismetInputLibrary|KeyIsGamepadKey Key))))

(fn ConstructionScript)

(fn UpdatePlayerAim
  (if (CallFunction|IsPlayerAlive)
    (if (Variables|Default|GetGamePadActive)
      (ThumbstickInput|UpdateThumbstickAim)
      (else
        (MouseInput|UpdateMouseAim)))))

(fn IsThumbstickAboveDeadZone
  (return (> (Math|Vector2D|Vector2DLength (Math|Vector2D|MakeVector2D (Input|AxisValues|GetThumbstickAimUp) (Input|AxisValues|GetThumbstickAimRight))) (Variables|ThumbstickInput|GetThumbstickDeadZone))))

(fn GetMouseVelocity
  (bind _returnvalue (Game|GetPlayerController 0))
  (bind (_deltax _deltay) (Class|PlayerController|GetInputMouseDelta _returnvalue))
  (return (/ (Math|Vector2D|MakeVector2D _deltax _deltay) (Utilities|Time|GetWorldDeltaSeconds))))

(fn IsMouseAboveDeadZone
  (return (> (Math|Vector2D|Vector2DLength (MouseInput|GetMouseVelocity)) (Variables|MouseInput|GetMouseDeadZone))))

(fn UpdateMouseAim
  (if (MouseInput|IsMouseAboveDeadZone)
    (Pawn|SetControlRotation (Game|GetPlayerController 0) (MouseInput|GetMouseAimDirection))))

(fn GetMouseAimDirection
  (bind _returnvalue (MouseInput|GetMouseVelocity))
  (return (Math|Interpolation|RInterpTo (Pawn|GetControlRotation (Game|GetPlayerController 0) :!class /Script/Engine.Controller) (Math|Rotator|MakeRotator 0.0 0.0 (Class|KismetMathLibrary|DegAtan2 (.x _returnvalue) (.y _returnvalue))) (Utilities|Time|GetWorldDeltaSeconds) (Variables|MouseInput|GetMouseSmoothStrengh))))

(fn GetThumbstickAimDirection
  (return (ThumbstickInput|ThumbStickDirectionProperties)))

(fn UpdateThumbstickAim
  (if (ThumbstickInput|IsThumbstickAboveDeadZone)
    (Pawn|SetControlRotation (Game|GetPlayerController 0) (ThumbstickInput|GetThumbstickAimDirection))))

(fn ThumbStickDirectionProperties
  (return (Math|Interpolation|RInterpTo (Pawn|GetControlRotation (Game|GetPlayerController 0) :!class /Script/Engine.Controller) (Math|Rotator|MakeRotator 0.0 0.0 (Class|KismetMathLibrary|DegAtan2 (Input|AxisValues|GetThumbstickAimRight) (Input|AxisValues|GetThumbstickAimUp))) (Utilities|Time|GetWorldDeltaSeconds) (Variables|ThumbstickInput|GetThumbStick%20SmoothStrengh))))

(fn StartFiringWeapon
  (if (CallFunction|IsPlayerAlive)
    (Components|Activation|Activate (Variables|Default|GetP_AssaultRifle_MF) false)
    ;[1 1 1] Play firing sound
    (bind _returnvalue (Audio|SpawnSound2D "/Game/Sounds/Weapon_AssaultRifle/Stereo/RifleFireLoop_Cue.RifleFireLoop_Cue" 1.0 1.0 0.0 0))
    (Variables|Default|SetWeaponFireSound _returnvalue)
    (CallFunction|WeaponTrace)
    (Utilities|Time|SetTimerbyFunctionName 0 "WeaponTrace" (Variables|Default|GetWeapon%20FireRate) true)))

(fn StopFiringWeapon
  (bind _weaponfiresound (Variables|Default|GetWeaponFireSound))
  (Components|Activation|Deactivate (Variables|Default|GetP_AssaultRifle_MF))
  ;[1 1 1] Stop Firing sound
  (Utilities|IsValid _weaponfiresound
    (:Is%20Valid
      (Audio|Components|Audio|Stop _weaponfiresound)
      (Utilities|Time|ClearTimerbyFunctionName 0 "WeaponTrace"))
    (:Is%20Not%20Valid
      _))
  (if (CallFunction|IsPlayerAlive)
    (Audio|SpawnSound2D "/Game/Sounds/Weapon_AssaultRifle/Stereo/RifleFireEnd_Cue.RifleFireEnd_Cue" 1.0 1.0 0.0 0)))

(fn DecreaseHealth
  (params (Damage%20Amount :type Float%20%28single-precision%29))
  (bind _output_get (Variables|PlayerProperties|SetHealth (Math|Float|Clamp(Float) (- (Variables|PlayerProperties|GetHealth) Damage%20Amount) 0.0 1e+02)))
  (return _output_get))

(fn IsPlayerAlive
  (return (not (Variables|PlayerProperties|GetDead))))

(fn WeaponTrace
  (bind _outhit (Collision|LineTraceByChannel (CallFunction|GetWeaponTraceStartLocation) (CallFunction|GetTraceEndLocation) "TraceTypeQuery1" false 0 "ForDuration"))
  (if (.bBlockingHit (Collision|BreakHitResult _outhit))
    (Game|Damage|ApplyDamage (.HitActor (Collision|BreakHitResult _outhit)) (Variables|Default|GetDamage%20per%20Shot) 0 0)))

(fn GetWeaponTraceStartLocation
  (return (Transformation|GetSocketLocation (Variables|Default|GetRifle) "MuzzleFlashSocket")))

(fn GetTraceEndLocation
  (return (+ (CallFunction|GetWeaponTraceStartLocation) (* (Math|Vector|GetForwardVector (Pawn|GetControlRotation :!class /Script/Engine.Pawn)) (Variables|Default|GetWeapon%20Range)))))

(fn IncreaseKills
  (Variables|PlayerProperties|SetKills (+ (Variables|PlayerProperties|GetKills) 1)))